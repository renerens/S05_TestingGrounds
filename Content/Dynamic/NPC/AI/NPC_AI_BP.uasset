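; AI controller for a guard NPC that runs the GuardBehaviour behavior tree with the PatrolBlackboardData blackboard.
; Perception updates set the blackboard's enemy key to sensed actors lacking the "Enemy" tag, and clear it when such an actor is not successfully sensed.
; Each tick it sets the controlled PatrollingGuard2's Aiming and Shooting flags according to whether a valid focus actor exists.
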(event OnTargetPerceptionUpdated(AIPerception)
  (params (Actor :type Actor%20Object%20Reference) (Stimulus :type AI%20Stimulus%20Structure))
  (bind _blackboardcomponent (Variables|Default|GetBlackBoardComponent))
  (bind _enemykey (Variables|Default|GetEnemyKey))
  (if (not (Actor|ActorHasTag Actor "Enemy"))
    (if (.bsuccessfullysensed Stimulus)
      (AI|Components|Blackboard|SetValueasObject _blackboardcomponent _enemykey Actor)
      (Development|PrintString "Setting Enemy")
      (else
        (AI|Components|Blackboard|ClearValue _blackboardcomponent _enemykey)
        (Development|PrintString "Clearing Enemy")))))

(event EventBeginPlay
  (bind _blackboardcomponent (Class|AIController|UseBlackboard "/Game/Dynamic/NPC/AI/PatrolBlackboardData.PatrolBlackboardData"))
  (AI|RunBehaviorTree "/Game/Dynamic/NPC/AI/GuardBehaviour.GuardBehaviour")
  (Variables|Default|SetBlackBoardComponent _blackboardcomponent))

(event EventTick
  (params (DeltaSeconds :type Float%20%28single-precision%29))
  (bind _returnvalue (Class|AIController|GetFocusActor))
  (bind _returnvalue_2 (Utilities|IsValid _returnvalue))
  (bind _aspatrolling_guard_2 (Utilities|Casting|CastToPatrollingGuard2 (Pawn|GetControlledPawn)))
  (Variables|/Game/Dynamic/NPC/Behaviour/PatrollingGuard2.PatrollingGuard2_C|SetAiming _aspatrolling_guard_2 _returnvalue_2)
  (Variables|/Game/Dynamic/NPC/Behaviour/PatrollingGuard2.PatrollingGuard2_C|SetShooting _aspatrolling_guard_2 _returnvalue_2))

(fn ConstructionScript)